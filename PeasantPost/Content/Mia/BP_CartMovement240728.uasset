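; Player-ridden delivery cart that runs along X and eases toward its LaneParent's Y on Tick.
; Boarding starts a stopped cart; delivery points stop it and spawn a starter parcel, while alert mode restarts it in negative direction and calls the postman's EnterGun.
; Blockades apply per-tick countdown knockback and slow floors halve travel and lane-change speed.
; Trigger boxes set the postman's lever flags and parcels' on-wagon state.
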(event `Reset Speed`
  (if (`self.AlertModeActive`)
    (set `self.CartSpeed` (`self.CartSpeed_AlertMode`))
    (else
      (set `self.CartSpeed` (`self.CartSpeed_DeliveryMode`)))))

(event `self.ReceiveTick`
  (params (DeltaSeconds :type "Float (single-precision)"))
  (bind (_returnvalue_x _returnvalue_y) (`KismetMathLibrary.BreakVector` (`self.K2_GetActorLocation`)))
  (bind (_returnvalue_x_2 _returnvalue_y_2 _returnvalue_z) (`KismetMathLibrary.BreakVector` (`self.K2_GetActorLocation`)))
  (bind (_returnvalue_x_3 _returnvalue_y_3) (`KismetMathLibrary.BreakVector` (`self.K2_GetActorLocation` (`self.laneParent`))))
  (bind (_returnvalue_x_4 _returnvalue_y_4) (`KismetMathLibrary.BreakVector` (`KismetMathLibrary.VInterpTo` (`KismetMathLibrary.MakeVector` _returnvalue_x_2 _returnvalue_y_2 _returnvalue_z) (`KismetMathLibrary.MakeVector` _returnvalue_x_2 _returnvalue_y_3 _returnvalue_z) DeltaSeconds (`self.changeLaneSpeed`))))
  (bind (_returnvalue_x_5 _returnvalue_y_5) (`KismetMathLibrary.BreakVector` (`SceneComponent.K2_GetComponentLocation` (`/Game/Mia/BP_Lanes.Plane` (`self.laneParent`)))))
  ;[0 0 0] If dead, can't move - reset level?
  (if (`self.IsDead`)
    (`KismetSystemLibrary.PrintString` "Cart is damaged beyond repair" true true (struct :`G` 0.66 :`B` 1.0 :`A` 1.0) 1.0)
    (else
      (if (== 0 (`self.cartState`))
        (set `self.xMovement` 0.0)
        (else
          (if (> (`self.knockbackNum`) 0.0)
            (set `self.xMovementTrue` (* (* -1 (`self.CartDirection`)) (* (`self.knockbackNum`) 0.25)))
            (set `self.knockbackNum` (- (`self.knockbackNum`) 1.0))
            (else
              ;[0 0 0] Continuous movement
              (set `self.xMovementTrue` (* (`self.CartSpeed`) (`self.CartDirection`)))))
          (if (`self.slowed`)
            (set `self.xMovement` (* 0.5 (`self.xMovementTrue`)))
            (set `self.changeLaneSpeed` (* 0.5 (`self.changeLaneSpeedTrue`)))
            (else
              (set `self.xMovement` (`self.xMovementTrue`))
              (set `self.changeLaneSpeed` (`self.changeLaneSpeedTrue`))))))
      (`KismetSystemLibrary.DelayUntilNextTick`)
      (`self.K2_SetActorLocation` (`KismetMathLibrary.MakeVector` (+ (`self.xMovement`) _returnvalue_x_2) _returnvalue_y_4 _returnvalue_z))
      (if (== _returnvalue_y _returnvalue_y_5)
        (set `self.isChangingLane` false)))))

(event `self.BoxCollider_Down.OnComponentBeginOverlap`
  (params (OverlappedComponent :type "PrimitiveComponent Object Reference") (OtherActor :type "Actor Object Reference") (OtherComp :type "PrimitiveComponent Object Reference") (OtherBodyIndex :type Integer) (bFromSweep :type Boolean) (SweepResult :type "HitResult Structure (by ref)"))
  ;[0 0 0] Checking if player is on the Right(Down) lever and changing bool
  (bind _asbp_postman (cast `/Game/Character/BP_Postman` OtherActor))
  (bind _output_get (set `/Game/Character/BP_Postman.onSwitchR` true _asbp_postman))
  (set `self.PlayerOnLeverR` _output_get)
  (set `self.direction` 1))

(event `self.BoxCollider_Down.OnComponentEndOverlap`
  (params (OverlappedComponent :type "PrimitiveComponent Object Reference") (OtherActor :type "Actor Object Reference") (OtherComp :type "PrimitiveComponent Object Reference") (OtherBodyIndex :type Integer))
  ;[0 0 0] Checking if player is on the Right(Down) lever and changing bool
  (bind _asbp_postman (cast `/Game/Character/BP_Postman` OtherActor))
  (set `/Game/Character/BP_Postman.onSwitchR` false _asbp_postman))

(event `self.BoxCollider_Cart.OnComponentBeginOverlap`
  (params (OverlappedComponent :type "PrimitiveComponent Object Reference") (OtherActor :type "Actor Object Reference") (OtherComp :type "PrimitiveComponent Object Reference") (OtherBodyIndex :type Integer) (bFromSweep :type Boolean) (SweepResult :type "HitResult Structure (by ref)"))
  ;[0 0 0] Checking if player is on Cart and changing bool
  (cast `/Game/Character/BP_Postman` OtherActor
    (:`then`
      (set `self.PlayerOnCart` true)
      (if (and (== (`self.cartState`) 0) (not (`self.makingDelivery`)))
        (`self.Reset Speed`)
        (set `self.cartState` 1)))
    (:`CastFailed`
      (bind _asbp_parcel (cast `/Game/Character/BP_Parcel` OtherActor))
      (set `/Game/Character/BP_Parcel.onWagon` true _asbp_parcel)
      (`KismetSystemLibrary.PrintString` "ON WAGON"))))

(event `self.BoxCollider_Up.OnComponentBeginOverlap`
  (params (OverlappedComponent :type "PrimitiveComponent Object Reference") (OtherActor :type "Actor Object Reference") (OtherComp :type "PrimitiveComponent Object Reference") (OtherBodyIndex :type Integer) (bFromSweep :type Boolean) (SweepResult :type "HitResult Structure (by ref)"))
  ;[0 0 0] Checking if player is on the Left(Up) lever and changing bool
  (bind _asbp_postman (cast `/Game/Character/BP_Postman` OtherActor))
  (bind _output_get (set `/Game/Character/BP_Postman.onSwitchL` true _asbp_postman))
  (set `self.PlayerOnLeverL` _output_get)
  (set `self.direction` -1))

(event `self.BoxCollider_Cart.OnComponentEndOverlap`
  (params (OverlappedComponent :type "PrimitiveComponent Object Reference") (OtherActor :type "Actor Object Reference") (OtherComp :type "PrimitiveComponent Object Reference") (OtherBodyIndex :type Integer))
  ;[0 0 0] Checking if player is on Cart and changing bool
  (cast `/Game/Character/BP_Postman` OtherActor
    (:`then`
      (set `self.PlayerOnCart` false))
    (:`CastFailed`
      (bind _asbp_parcel (cast `/Game/Character/BP_Parcel` OtherActor))
      (set `/Game/Character/BP_Parcel.onWagon` false _asbp_parcel))))

(event `self.BoxCollider_Up.OnComponentEndOverlap`
  (params (OverlappedComponent :type "PrimitiveComponent Object Reference") (OtherActor :type "Actor Object Reference") (OtherComp :type "PrimitiveComponent Object Reference") (OtherBodyIndex :type Integer))
  ;[0 0 0] Checking if player is on the Left(Up) lever and changing bool
  (bind _asbp_postman (cast `/Game/Character/BP_Postman` OtherActor))
  (set `/Game/Character/BP_Postman.onSwitchL` false _asbp_postman))

(event `Activate Alert Mode`
  (if (== (`self.cartState`) 0)
    (bind _output_get (set `self.cartState` -1))
    (set `self.CartDirection` _output_get)
    (`self.Reset Speed`)
    (bind _returnvalue (`GameplayStatics.GetActorOfClass` "/Game/Character/BP_Postman.BP_Postman_C"))
    (`/Game/Character/BP_Postman.Enter Gun` _returnvalue)))

(event `Parcel Placed On Wagon`
  ;[0 0 0] MAIN parcel is placed onto wagon
)

(event `self.Plane .OnComponentBeginOverlap`
  (params (OverlappedComponent :type "PrimitiveComponent Object Reference") (OtherActor :type "Actor Object Reference") (OtherComp :type "PrimitiveComponent Object Reference") (OtherBodyIndex :type Integer) (bFromSweep :type Boolean) (SweepResult :type "HitResult Structure (by ref)"))
  (bind (_returnvalue_x _returnvalue_y _returnvalue_z) (`KismetMathLibrary.BreakVector` (`SceneComponent.K2_GetComponentLocation` (`self.Parcel_Cube`))))
  ;[0 0 0] MAIN parcel is placed onto wagon
  (if false
    (bind _asbp_parcel (cast `/Game/Character/BP_Parcel` OtherActor))
    (if (and (`/Game/Character/BP_Parcel.isMainParcel` _asbp_parcel) (== (`self.cartState`) 0))
      (bind _output_get (set `self.cartState` -1))
      (set `self.CartDirection` _output_get)
      (`self.Reset Speed`))
    (else
      ;[0.01 0.01 0.01] reaches delivery point
      (if (== (`GameplayStatics.GetObjectClass` OtherActor) "/Game/Mia/BP_Delivery.BP_Delivery_C")
        (set `self.cartState` 0)
        (bind _returnvalue (`|SpawnActorFromClass` "/Game/Character/BP_Parcel.BP_Parcel_C" (`KismetMathLibrary.MakeTransform` (`KismetMathLibrary.MakeVector` _returnvalue_x _returnvalue_y _returnvalue_z)) "Undefined" "MultiplyWithRoot" null null))
        (bind _output_get_2 (set `/Game/Character/BP_Parcel.isStarterParcel` true _returnvalue))
        (set `self.makingDelivery` _output_get_2)))))

(event `self.Plane .OnComponentEndOverlap`
  (params (OverlappedComponent :type "PrimitiveComponent Object Reference") (OtherActor :type "Actor Object Reference") (OtherComp :type "PrimitiveComponent Object Reference") (OtherBodyIndex :type Integer))
  ;[0 0 0] MAIN parcel is placed onto wagon
  ;[0.01 0.01 0.01] reaches delivery point
  (if (== (`GameplayStatics.GetObjectClass` OtherActor) "/Game/Mia/BP_Delivery.BP_Delivery_C")
    (set `self.makingDelivery` false)))

(event `self.Knockback Box.OnComponentBeginOverlap`
  (params (OverlappedComponent :type "PrimitiveComponent Object Reference") (OtherActor :type "Actor Object Reference") (OtherComp :type "PrimitiveComponent Object Reference") (OtherBodyIndex :type Integer) (bFromSweep :type Boolean) (SweepResult :type "HitResult Structure (by ref)"))
  (bind _returnvalue (`GameplayStatics.GetObjectClass` OtherActor))
  ;[0.063 0.063 0.063] hits blockade
  (if (== _returnvalue "/Game/Mia/BP_Blockade.BP_Blockade_C")
    (`KismetSystemLibrary.PrintString` "DAMAGE")
    (set `self.isChangingLane` true)
    (bind _asbp_blockade (cast `/Game/Mia/BP_Blockade` OtherActor))
    (set `self.knockbackNum` (`/Game/Mia/BP_Blockade.knockbackAmount` _asbp_blockade))
    (else
      ;[0.063 0.063 0.063] hits slow floor
      (if (== _returnvalue "/Game/Mia/BP_Slow_Floor.BP_Slow_Floor_C")
        (`KismetSystemLibrary.PrintString` "SLOW FLOOR")
        (set `self.slowed` true)))))

(event `self.Knockback Box.OnComponentEndOverlap`
  (params (OverlappedComponent :type "PrimitiveComponent Object Reference") (OtherActor :type "Actor Object Reference") (OtherComp :type "PrimitiveComponent Object Reference") (OtherBodyIndex :type Integer))
  ;[0.063 0.063 0.063] hits slow floor
  (if (<= (`KismetArrayLibrary.Array_Length` (`PrimitiveComponent.GetOverlappingActors` (`self.Knockback Box`) "/Game/Mia/BP_Slow_Floor.BP_Slow_Floor_C")) 0)
    (`KismetSystemLibrary.PrintString` "NO FLOOR")
    (set `self.slowed` false)))

(fn `UserConstructionScript`)