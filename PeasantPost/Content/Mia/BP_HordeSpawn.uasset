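; Horde spawn trigger that spawns groups of enemies and their patrol routes when BP_CartMovement overlaps its Plane, then destroys itself.
; BeginPlay derives the Y spread from the SpawnHigh and SpawnLow markers, centred on the Plane.
; Each of four per-type counts drives a loop spawning at random offsets.
; The loop index, not the count's type, picks chameleon, goblin archer or mud monster, defaulting to beetleowl.
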(event `self.ReceiveBeginPlay`
  (bind _plane (`self.Plane`))
  (bind _spawnyminmax (`self.spawnYminmax`))
  (bind (_returnvalue_x _returnvalue_y) (`KismetMathLibrary.BreakVector` (`SceneComponent.K2_GetComponentLocation` _plane)))
  (bind (_returnvalue_x_2 _returnvalue_y_2) (`KismetMathLibrary.BreakVector` (`SceneComponent.K2_GetComponentLocation` (`self.spawnHigh`))))
  (bind (_returnvalue_x_3 _returnvalue_y_3) (`KismetMathLibrary.BreakVector` (`SceneComponent.K2_GetComponentScale` _plane)))
  (bind (_returnvalue_x_4 _returnvalue_y_4) (`KismetMathLibrary.BreakVector` (`SceneComponent.K2_GetComponentLocation` (`self.spawnLow`))))
  (set `self.enemyTotalNum` (+ (`self.chameleonNum`) (`self.goblinNum`) (`self.mudNum`) (`self.beetlebugNum`)))
  (if (> _returnvalue_y_2 _returnvalue_y_4)
    (set `self.spawnYminmax` (/ (- _returnvalue_y_2 _returnvalue_y_4) 2.0))
    (else
      (set `self.spawnYminmax` (/ (- _returnvalue_y_4 _returnvalue_y_2) 2.0))))
  (set `self.spawnYtrue` _returnvalue_y)
  (set `self.spawnXtrue` _returnvalue_x)
  (set `self.spawnYmin` (- _returnvalue_y _spawnyminmax))
  (set `self.spawnYmax` (+ _spawnyminmax _returnvalue_y))
  (set `self.spawnDivider` _returnvalue_y_3))

(event `self.Plane.OnComponentBeginOverlap`
  (params (OverlappedComponent :type "PrimitiveComponent Object Reference") (OtherActor :type "Actor Object Reference") (OtherComp :type "PrimitiveComponent Object Reference") (OtherBodyIndex :type Integer) (bFromSweep :type Boolean) (SweepResult :type "HitResult Structure (by ref)"))
  (bind _spawnyminmax (`self.spawnYminmax`))
  (if (== (`GameplayStatics.GetObjectClass` OtherActor) "/Game/Mia/BP_CartMovement.BP_CartMovement_C")
    (bind _asbp_cart_movement (cast `/Game/Mia/BP_CartMovement` OtherActor))
    (if (`/Game/Mia/BP_CartMovement.AlertModeActive` _asbp_cart_movement)
      _
      (else
        _))
    (for _array_element (`|MakeArray` (`self.chameleonNum`) (`self.goblinNum`) (`self.mudNum`) (`self.beetlebugNum`))
      (set `self.spawnDivider` (/ (- (`self.spawnYmax`) (`self.spawnYmin`)) _array_element))
      (for _index (range (+ _array_element 1))
        (set `self.spawnYcurrent` (+ (`self.spawnYtrue`) (`KismetMathLibrary.RandomFloatInRange` (* -1.0 _spawnyminmax) _spawnyminmax)))
        (`KismetSystemLibrary.PrintString` (`KismetStringLibrary.Conv_DoubleToString` _spawnyminmax))
        (set `self.spawnX` (+ (`self.spawnXtrue`) (`KismetMathLibrary.RandomFloatInRange` -500.0 -200.0)))
        (set `self.spawnVector` (`KismetMathLibrary.MakeVector` (`self.spawnX`) (`self.spawnYcurrent`) 10.0))
        (switch `int` _index
          (:`Default`
            (bind _returnvalue (`|SpawnActorFromClass` "/Game/Enemies/BeetleowlBug/BP_EnemyBeetleowlTrueChild.BP_EnemyBeetleowlTrueChild_C" (`KismetMathLibrary.MakeTransform` (`self.spawnVector`)) "AdjustIfPossibleButAlwaysSpawn" "MultiplyWithRoot" null "NewEnumerator1" null :!label _label))
            (`/Game/Enemies/Enemy_Basic/BP_EnemyBasicChar.GetPatrolRoute` _returnvalue))
          (:`0`
            (bind _returnvalue_2 (`|SpawnActorFromClass` "/Game/Enemies/Chameleon/BP_EnemyChameleon.BP_EnemyChameleon_C" (`KismetMathLibrary.MakeTransform` (`self.spawnVector`)) "AdjustIfPossibleButAlwaysSpawn" "MultiplyWithRoot" null "NewEnumerator3" null))
            (`/Game/Enemies/Enemy_Basic/BP_EnemyBasicChar.GetPatrolRoute` _returnvalue_2))
          (:`1`
            (bind _returnvalue_3 (`|SpawnActorFromClass` "/Game/Enemies/GoblinArcher/BP_EnemyGoblinArcher.BP_EnemyGoblinArcher_C" (`KismetMathLibrary.MakeTransform` (`self.spawnVector`)) "AdjustIfPossibleButAlwaysSpawn" "MultiplyWithRoot" null "NewEnumerator4" null))
            (`/Game/Enemies/Enemy_Basic/BP_EnemyBasicChar.GetPatrolRoute` _returnvalue_3))
          (:`2`
            (bind _returnvalue_4 (`|SpawnActorFromClass` "/Game/Enemies/MudMonster/BP_EnemyMudMonster.BP_EnemyMudMonster_C" (`KismetMathLibrary.MakeTransform` (`self.spawnVector`)) "AdjustIfPossibleButAlwaysSpawn" "MultiplyWithRoot" null "NewEnumerator2" null))
            (`/Game/Enemies/AI/BPI_EnemyAI.GetPatrolRoute` _returnvalue_4))
          (:`3`
            (goto _label)))))
    (`self.K2_DestroyActor`)))

(fn `UserConstructionScript`)