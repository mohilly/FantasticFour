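; Delivery cart that travels along X and glides in Y toward its LaneParent's lane.
; Tick drives movement from CartState, CartSpeed and CartDirection, with blockade hits causing a decaying knockback.
; Overlaps start the cart when the main parcel lands, change state at delivery points, and flag the postman on cart or lane levers.
; Slow floors only set a flag, as the speed-halving logic is disconnected.
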(event `Reset Speed`
  (if (`self.AlertModeActive`)
    (set `self.CartSpeed` (`self.CartSpeed_AlertMode`))
    (else
      (set `self.CartSpeed` (`self.CartSpeed_DeliveryMode`)))))

(event `self.ReceiveTick`
  (params (DeltaSeconds :type "Float (single-precision)"))
  (bind (_returnvalue_x _returnvalue_y) (`KismetMathLibrary.BreakVector` (`self.K2_GetActorLocation`)))
  (bind (_returnvalue_x_2 _returnvalue_y_2 _returnvalue_z) (`KismetMathLibrary.BreakVector` (`self.K2_GetActorLocation`)))
  (bind (_returnvalue_x_3 _returnvalue_y_3 _returnvalue_z_2) (`KismetMathLibrary.BreakVector` (`self.K2_GetActorLocation`)))
  (bind (_returnvalue_x_4 _returnvalue_y_4 _returnvalue_z_3) (`KismetMathLibrary.BreakVector` (`self.K2_GetActorLocation`)))
  (bind (_returnvalue_x_5 _returnvalue_y_5) (`KismetMathLibrary.BreakVector` (`self.K2_GetActorLocation` (`self.laneParent`))))
  (bind (_returnvalue_x_6 _returnvalue_y_6) (`KismetMathLibrary.BreakVector` (`KismetMathLibrary.VInterpTo` (`KismetMathLibrary.MakeVector` _returnvalue_x_4 _returnvalue_y_4 _returnvalue_z_3) (`KismetMathLibrary.MakeVector` _returnvalue_x_4 _returnvalue_y_5 _returnvalue_z_3) DeltaSeconds (`self.changeLaneSpeed`))))
  (bind (_returnvalue_x_7 _returnvalue_y_7) (`KismetMathLibrary.BreakVector` (`SceneComponent.K2_GetComponentLocation` (`/Game/Mia/BP_Lanes.Plane` (`self.laneParent`)))))
  ;[0 0 0] If dead, can't move - reset level?
  (if (`self.IsDead`)
    (`KismetSystemLibrary.PrintString` "Cart is damaged beyond repair" true true (struct :`G` 0.66 :`B` 1.0 :`A` 1.0) 1.0)
    (else
      (if (== 0 (`self.cartState`))
        _
        (elif (> (`self.knockbackNum`) 0.0)
          (`self.K2_SetActorLocation` (`KismetMathLibrary.MakeVector` (+ (* (* -1 (`self.CartDirection`)) (* (`self.knockbackNum`) 0.25)) _returnvalue_x_2) _returnvalue_y_2 _returnvalue_z))
          (set `self.knockbackNum` (- (`self.knockbackNum`) 1.0))
          (else
            ;[0 0 0] Continuous movement
            (`self.K2_SetActorLocation` (`KismetMathLibrary.MakeVector` (+ (* (`self.CartSpeed`) (`self.CartDirection`)) _returnvalue_x_3) _returnvalue_y_3 _returnvalue_z_2)))))
      (`self.K2_SetActorLocation` (`KismetMathLibrary.MakeVector` _returnvalue_x_4 _returnvalue_y_6 _returnvalue_z_3))
      (if (== _returnvalue_y _returnvalue_y_7)
        (set `self.isChangingLane` false)))))

(event `self.BoxCollider_Down.OnComponentBeginOverlap`
  (params (OverlappedComponent :type "PrimitiveComponent Object Reference") (OtherActor :type "Actor Object Reference") (OtherComp :type "PrimitiveComponent Object Reference") (OtherBodyIndex :type Integer) (bFromSweep :type Boolean) (SweepResult :type "HitResult Structure (by ref)"))
  ;[0 0 0] Checking if player is on the Right(Down) lever and changing bool
  (bind _asbp_postman (cast `/Game/Character/BP_Postman` OtherActor))
  (bind _output_get (set `/Game/Character/BP_Postman.onSwitchR` true _asbp_postman))
  (set `self.PlayerOnLeverR` _output_get)
  (set `self.direction` 1))

(event `self.BoxCollider_Down.OnComponentEndOverlap`
  (params (OverlappedComponent :type "PrimitiveComponent Object Reference") (OtherActor :type "Actor Object Reference") (OtherComp :type "PrimitiveComponent Object Reference") (OtherBodyIndex :type Integer))
  ;[0 0 0] Checking if player is on the Right(Down) lever and changing bool
  (bind _asbp_postman (cast `/Game/Character/BP_Postman` OtherActor))
  (set `/Game/Character/BP_Postman.onSwitchR` false _asbp_postman))

(event `self.BoxCollider_Cart.OnComponentBeginOverlap`
  (params (OverlappedComponent :type "PrimitiveComponent Object Reference") (OtherActor :type "Actor Object Reference") (OtherComp :type "PrimitiveComponent Object Reference") (OtherBodyIndex :type Integer) (bFromSweep :type Boolean) (SweepResult :type "HitResult Structure (by ref)"))
  ;[0 0 0] Checking if player is on Cart and changing bool
  (cast `/Game/Character/BP_Postman` OtherActor
    (:`then`
      (set `self.PlayerOnCart` true)
      (`KismetSystemLibrary.PrintString` "You can steer"))
    (:`CastFailed`
      _))
  (cast `/Game/Character/BP_Parcel` OtherActor))

(event `self.BoxCollider_Up.OnComponentBeginOverlap`
  (params (OverlappedComponent :type "PrimitiveComponent Object Reference") (OtherActor :type "Actor Object Reference") (OtherComp :type "PrimitiveComponent Object Reference") (OtherBodyIndex :type Integer) (bFromSweep :type Boolean) (SweepResult :type "HitResult Structure (by ref)"))
  ;[0 0 0] Checking if player is on the Left(Up) lever and changing bool
  (bind _asbp_postman (cast `/Game/Character/BP_Postman` OtherActor))
  (bind _output_get (set `/Game/Character/BP_Postman.onSwitchL` true _asbp_postman))
  (set `self.PlayerOnLeverL` _output_get)
  (set `self.direction` -1))

(event `self.BoxCollider_Cart.OnComponentEndOverlap`
  (params (OverlappedComponent :type "PrimitiveComponent Object Reference") (OtherActor :type "Actor Object Reference") (OtherComp :type "PrimitiveComponent Object Reference") (OtherBodyIndex :type Integer))
  ;[0 0 0] Checking if player is on Cart and changing bool
  (cast `/Game/Character/BP_Postman` OtherActor)
  (set `self.PlayerOnCart` false)
  (`KismetSystemLibrary.PrintString` "Not able to steer"))

(event `self.BoxCollider_Up.OnComponentEndOverlap`
  (params (OverlappedComponent :type "PrimitiveComponent Object Reference") (OtherActor :type "Actor Object Reference") (OtherComp :type "PrimitiveComponent Object Reference") (OtherBodyIndex :type Integer))
  ;[0 0 0] Checking if player is on the Left(Up) lever and changing bool
  (bind _asbp_postman (cast `/Game/Character/BP_Postman` OtherActor))
  (set `/Game/Character/BP_Postman.onSwitchL` false _asbp_postman))

(event `Parcel Placed On Wagon`
  ;[0 0 0] MAIN parcel is placed onto wagon
)

(event `self.Plane .OnComponentBeginOverlap`
  (params (OverlappedComponent :type "PrimitiveComponent Object Reference") (OtherActor :type "Actor Object Reference") (OtherComp :type "PrimitiveComponent Object Reference") (OtherBodyIndex :type Integer) (bFromSweep :type Boolean) (SweepResult :type "HitResult Structure (by ref)"))
  (bind _returnvalue (`GameplayStatics.GetObjectClass` OtherActor))
  ;[0 0 0] MAIN parcel is placed onto wagon
  (if (== _returnvalue "/Game/Character/BP_Parcel.BP_Parcel_C")
    (bind _asbp_parcel (cast `/Game/Character/BP_Parcel` OtherActor))
    (if (and (`/Game/Character/BP_Parcel.isMainParcel` _asbp_parcel) (== (`self.cartState`) 0))
      (bind _output_get (set `self.cartState` -1))
      (set `self.CartDirection` _output_get)
      (set `self.CartSpeed` (`self.CartSpeed_AlertMode`)))
    (else
      ;[0.01 0.01 0.01] reaches delivery point
      (if (== _returnvalue "/Game/Mia/BP_Delivery.BP_Delivery_C")
        (set `self.cartState` 0)))))

(event `self.Plane .OnComponentEndOverlap`
  (params (OverlappedComponent :type "PrimitiveComponent Object Reference") (OtherActor :type "Actor Object Reference") (OtherComp :type "PrimitiveComponent Object Reference") (OtherBodyIndex :type Integer))
  ;[0 0 0] MAIN parcel is placed onto wagon
  ;[0.01 0.01 0.01] reaches delivery point
  (if (== (`GameplayStatics.GetObjectClass` OtherActor) "/Game/Mia/BP_Delivery.BP_Delivery_C")
    (set `self.cartState` 1)))

(event `self.Knockback Box.OnComponentBeginOverlap`
  (params (OverlappedComponent :type "PrimitiveComponent Object Reference") (OtherActor :type "Actor Object Reference") (OtherComp :type "PrimitiveComponent Object Reference") (OtherBodyIndex :type Integer) (bFromSweep :type Boolean) (SweepResult :type "HitResult Structure (by ref)"))
  (bind _returnvalue (`GameplayStatics.GetObjectClass` OtherActor))
  ;[0.063 0.063 0.063] hits blockade
  (if (== _returnvalue "/Game/Mia/BP_Blockade.BP_Blockade_C")
    (`KismetSystemLibrary.PrintString` "DAMAGE")
    (set `self.isChangingLane` true)
    (bind _asbp_blockade (cast `/Game/Mia/BP_Blockade` OtherActor))
    (set `self.knockbackNum` (`/Game/Mia/BP_Blockade.knockbackAmount` _asbp_blockade))
    (`KismetSystemLibrary.PrintString` (`KismetStringLibrary.Conv_DoubleToString` (`self.knockbackNum`)))
    (else
      ;[0.063 0.063 0.063] hits slow floor
      (if (== _returnvalue "/Game/Mia/BP_Slow_Floor.BP_Slow_Floor_C")
        (`KismetSystemLibrary.PrintString` "SLOW FLOOR")
        (set `self.slowed` true)))))

(event `self.Knockback Box.OnComponentEndOverlap`
  (params (OverlappedComponent :type "PrimitiveComponent Object Reference") (OtherActor :type "Actor Object Reference") (OtherComp :type "PrimitiveComponent Object Reference") (OtherBodyIndex :type Integer))
  ;[0.063 0.063 0.063] hits slow floor
  (if (== (`GameplayStatics.GetObjectClass` (stale `self.Knockback Box.OnComponentBeginOverlap` OtherActor)) "/Game/Mia/BP_Slow_Floor.BP_Slow_Floor_C")
    (`KismetSystemLibrary.PrintString` "NO FLOOR")
    (set `self.slowed` false)))

(fn `UserConstructionScript`)