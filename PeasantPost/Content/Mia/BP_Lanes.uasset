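; BP_Lanes is a lane actor that owns a cart and can shift sideways by whole lane widths.
; On BeginPlay it spawns a BP_CartMovement offset along X from WagonSpawn and links itself as parent.
; MoveLane range-checks the lane index, then moves the actor along Y using the Plane's bounds.
; Overlap events at WagonSpawn and ParcelSpawn set CartState to 0; parcel spawning logic is unconnected.
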(event `self.ReceiveBeginPlay`
  (bind (_returnvalue_x _returnvalue_y _returnvalue_z) (`KismetMathLibrary.BreakVector` (`SceneComponent.K2_GetComponentLocation` (`self.Wagon Spawn`))))
  (bind _returnvalue (`|SpawnActorFromClass` "/Game/Mia/BP_CartMovement.BP_CartMovement_C" (`KismetMathLibrary.MakeTransform` (`KismetMathLibrary.MakeVector` (+ (* (`self.spawn Distance`) -1.0) _returnvalue_x) _returnvalue_y _returnvalue_z)) "AdjustIfPossibleButAlwaysSpawn" "MultiplyWithRoot" null null))
  (bind _output_get (set `self.wagonChild` _returnvalue))
  (set `/Game/Mia/BP_CartMovement.laneParent` self _output_get))

(event `Move Lane`
  (params (direction :type Integer))
  (bind (_returnvalue_x _returnvalue_y _returnvalue_z) (`KismetMathLibrary.BreakVector` (`self.K2_GetActorLocation` self)))
  (bind _returnvalue (+ (`self.laneNum`) direction))
  (if (`KismetMathLibrary.InRange_IntInt` _returnvalue (`self.laneNumMin`) (`self.laneNumMax`))
    (set `self.laneNum` _returnvalue)
    (`self.K2_SetActorTransform` (`KismetMathLibrary.MakeTransform` (`KismetMathLibrary.MakeVector` _returnvalue_x (+ _returnvalue_y (* 2.0 (* direction (.y (`.BoxExtent` (`KismetSystemLibrary.GetComponentBounds` (`self.Plane`))))))) _returnvalue_z) (`self.K2_GetActorRotation` self) (`self.GetActorScale3D` self)))))

(event `self.Parcel Spawn.OnComponentBeginOverlap`
  (params (OverlappedComponent :type "PrimitiveComponent Object Reference") (OtherActor :type "Actor Object Reference") (OtherComp :type "PrimitiveComponent Object Reference") (OtherBodyIndex :type Integer) (bFromSweep :type Boolean) (SweepResult :type "HitResult Structure (by ref)"))
  (bind _output_get (set `self.overlappedCart` OtherActor))
  (bind _asbp_cart_movement (cast `/Game/Mia/BP_CartMovement` _output_get))
  (set `/Game/Mia/BP_CartMovement.cartState` 0 _asbp_cart_movement))

(event `self.Wagon Spawn.OnComponentBeginOverlap`
  (params (OverlappedComponent :type "PrimitiveComponent Object Reference") (OtherActor :type "Actor Object Reference") (OtherComp :type "PrimitiveComponent Object Reference") (OtherBodyIndex :type Integer) (bFromSweep :type Boolean) (SweepResult :type "HitResult Structure (by ref)"))
  (if (== (`self.wagonChild`) OtherActor)
    (bind _asbp_cart_movement (cast `/Game/Mia/BP_CartMovement` OtherActor))
    (if (== (`/Game/Mia/BP_CartMovement.cartState` _asbp_cart_movement) -1)
      (set `/Game/Mia/BP_CartMovement.cartState` 0 _asbp_cart_movement))))

(fn `UserConstructionScript`)