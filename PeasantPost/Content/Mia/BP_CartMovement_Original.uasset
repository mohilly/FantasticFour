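; Cart actor that moves continuously along local X and can be steered sideways by the player standing on its levers.
; Overlap boxes on the cart and two levers set flags when BP_Postman enters or leaves.
; Tick offsets the Plane component by CartSpeed and, while the player is aboard, nudges it along Y by the active lever, right taking priority.
; When IsDead is set, movement stops and only a debug message prints.
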(event `self.ReceiveTick`
  (params (DeltaSeconds :type "Float (single-precision)"))
  ;[0 0 0] If dead, can't move - reset level?
  (if (`self.IsDead`)
    (`KismetSystemLibrary.PrintString` "Cart is damaged beyond repair" true true (struct :`G` 0.66 :`B` 1.0 :`A` 1.0) 1.0)
    (else
      ;[0 0 0] Continuos movement to the right
      (`SceneComponent.K2_AddLocalOffset` (`self.Plane `) (`KismetMathLibrary.MakeVector` (* DeltaSeconds (`self.CartSpeed`))) false false)
      ;[0 0 0] Enable Near-Far movement once player is on the cart
      (if (`self.PlayerOnCart`)
        (if (`self.PlayerOnLeverR`)
          (`SceneComponent.K2_AddLocalOffset` (`self.Plane `) (`KismetMathLibrary.MakeVector` 0.0 (* DeltaSeconds 20.0)) false false)
          (elif (`self.PlayerOnLeverL`)
            (`SceneComponent.K2_AddLocalOffset` (`self.Plane `) (`KismetMathLibrary.MakeVector` 0.0 (* DeltaSeconds -20.0)) false false)))))))

(event `self.BoxCollider_Down.OnComponentBeginOverlap`
  (params (OverlappedComponent :type "PrimitiveComponent Object Reference") (OtherActor :type "Actor Object Reference") (OtherComp :type "PrimitiveComponent Object Reference") (OtherBodyIndex :type Integer) (bFromSweep :type Boolean) (SweepResult :type "HitResult Structure (by ref)"))
  ;[0 0 0] Checking if player is on the Right(Down) lever and changing bool
  (cast `/Game/Character/BP_Postman` OtherActor)
  (set `self.PlayerOnLeverR` true))

(event `self.BoxCollider_Cart.OnComponentBeginOverlap`
  (params (OverlappedComponent :type "PrimitiveComponent Object Reference") (OtherActor :type "Actor Object Reference") (OtherComp :type "PrimitiveComponent Object Reference") (OtherBodyIndex :type Integer) (bFromSweep :type Boolean) (SweepResult :type "HitResult Structure (by ref)"))
  ;[0 0 0] Checking if player is on Cart and changing bool
  (cast `/Game/Character/BP_Postman` OtherActor)
  (set `self.PlayerOnCart` true)
  (`KismetSystemLibrary.PrintString` "You can steer"))

(event `self.BoxCollider_Down.OnComponentEndOverlap`
  (params (OverlappedComponent :type "PrimitiveComponent Object Reference") (OtherActor :type "Actor Object Reference") (OtherComp :type "PrimitiveComponent Object Reference") (OtherBodyIndex :type Integer))
  ;[0 0 0] Checking if player is on the Right(Down) lever and changing bool
  (cast `/Game/Character/BP_Postman` OtherActor)
  (set `self.PlayerOnLeverR` false))

(event `self.BoxCollider_Cart.OnComponentEndOverlap`
  (params (OverlappedComponent :type "PrimitiveComponent Object Reference") (OtherActor :type "Actor Object Reference") (OtherComp :type "PrimitiveComponent Object Reference") (OtherBodyIndex :type Integer))
  ;[0 0 0] Checking if player is on Cart and changing bool
  (cast `/Game/Character/BP_Postman` OtherActor)
  (set `self.PlayerOnCart` false)
  (`KismetSystemLibrary.PrintString` "Not able to steer"))

(event `self.BoxCollider_Up.OnComponentBeginOverlap`
  (params (OverlappedComponent :type "PrimitiveComponent Object Reference") (OtherActor :type "Actor Object Reference") (OtherComp :type "PrimitiveComponent Object Reference") (OtherBodyIndex :type Integer) (bFromSweep :type Boolean) (SweepResult :type "HitResult Structure (by ref)"))
  ;[0 0 0] Checking if player is on the Left(Up) lever and changing bool
  (cast `/Game/Character/BP_Postman` OtherActor)
  (set `self.PlayerOnLeverL` true))

(event `self.BoxCollider_Up.OnComponentEndOverlap`
  (params (OverlappedComponent :type "PrimitiveComponent Object Reference") (OtherActor :type "Actor Object Reference") (OtherComp :type "PrimitiveComponent Object Reference") (OtherBodyIndex :type Integer))
  ;[0 0 0] Checking if player is on the Left(Up) lever and changing bool
  (cast `/Game/Character/BP_Postman` OtherActor)
  (set `self.PlayerOnLeverL` false))

(fn `UserConstructionScript`)