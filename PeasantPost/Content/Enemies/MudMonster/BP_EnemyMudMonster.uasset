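; BP_EnemyMudMonster is the mud monster enemy, a character Blueprint that defers BeginPlay, Tick and construction to its parent class.
; It supplies its own SetMovementSpeed, mapping a speed tier from idle to fast onto the CharacterMovement max walk speed.
; GetIdealRange reports zero attack and defend radii.
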(event `self.ReceiveBeginPlay`
  (`parent.ReceiveBeginPlay`))

(event `self.ReceiveTick`
  (params (DeltaSeconds :type "Float (single-precision)"))
  (`parent.ReceiveTick` DeltaSeconds))

(fn `GetIdealRange`
  (returns (AttackRadius :type "Float (double-precision)") (DefendRadius :type "Float (double-precision)"))
  (return 0.0 0.0))

(fn `SetMovementSpeed`
  (params (Speed :type "/Game/Enemies/AI/ENUMs/E_MovementSpeed Enum" :default "NewEnumerator0"))
  (returns (SpeedValue :type "Float (double-precision)"))
  (set `CharacterMovementComponent.MaxWalkSpeed` (select `/Game/Enemies/AI/ENUMs/E_MovementSpeed` Speed :`NewEnumerator1` 10.0 :`NewEnumerator2` 50.0 :`NewEnumerator3` 100.0 :!type "Float (single-precision)") (`self.CharacterMovement`))
  (return 0.0))

(fn `UserConstructionScript`
  (`parent.UserConstructionScript`))