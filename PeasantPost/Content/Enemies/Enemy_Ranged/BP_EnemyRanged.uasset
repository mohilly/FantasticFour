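; Ranged enemy character with a sprite, driven by the basic enemy AI controller, with an unfinished attack.
; Attack flags itself as attacking, debug-traces visibility to the controller's target and fires OnAttackEnd, with no hit response or damage wired.
; Helper functions map speed tiers to walk speed and supply fixed attack and defend radii, while the patrol route getter is empty.
; BeginPlay sets the moving flag once and zeroes the sprite's world rotation.
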(event `self.ReceiveBeginPlay`
  ;[0 0 0] Checking if is moving
  (if (`NavMovementComponent.IsMovingOnGround` (`self.CharacterMovement`))
    (set `self.IsMoving` true)
    (else
      (set `self.IsMoving` false)))
  ;[0 0 0] Trying to turn sprite to camera - might be fucking up the rotation of the animation (!)
  (`SceneComponent.K2_SetWorldRotation` :`self` (`self.Sprite`)))

(event `/Game/Enemies/AI/BPI_EnemyAI.Attack`
  (set `self.IsAttacking` true)
  (bind _asbp_aic_enemy_basic (cast `/Game/Enemies/AI/AIControllers/BP_AIC_EnemyBasic` (`AIBlueprintHelperLibrary.GetAIController` self)))
  (bind _attack_target (`/Game/Enemies/AI/AIControllers/BP_AIC_EnemyBasic.Attack Target` _asbp_aic_enemy_basic)
    (:`then`
      (bind (_outhit _returnvalue) (`KismetSystemLibrary.LineTraceSingle` :`Start` (`self.K2_GetActorLocation` self) :`End` (`self.K2_GetActorLocation` _attack_target) :`TraceChannel` "TraceTypeQuery1" :`DrawDebugType` "ForDuration"))
      (if _returnvalue
        _
        (else
          _))
      (`self.OnAttackEnd`))
    (:`else`)))

(fn `GetIdealRange`
  (returns (AttackRadius :type "Float (double-precision)") (DefendRadius :type "Float (double-precision)"))
  (return 300.0 500.0))

(fn `GetPatrolRoute`
  (returns (PatrolRoute :type "/Game/Enemies/AI/BP_PatrolRoute Object Reference"))
  (return null))

(fn `SetMovementSpeed`
  (params (Speed :type "/Game/Enemies/AI/ENUMs/E_MovementSpeed Enum" :default "NewEnumerator0"))
  (returns (SpeedValue :type "Float (double-precision)"))
  (set `CharacterMovementComponent.MaxWalkSpeed` (select `/Game/Enemies/AI/ENUMs/E_MovementSpeed` Speed :`NewEnumerator1` 200.0 :`NewEnumerator2` 350.0 :`NewEnumerator3` 550.0 :!type "Float (single-precision)") (`self.CharacterMovement`))
  (return 0.0))

(fn `UserConstructionScript`
  (`parent.UserConstructionScript`))