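; BP_EnemyMudMonster is a mud monster enemy character that deals melee damage to the target chosen by its AI controller.
; Attack reads AttackTarget from BP_AIC_MudMonster_Child, sends it a damage message, then clears IsAttacking and signals attack end after a short delay.
; SetMovementSpeed maps speed states to walk speeds, while begin play, tick and death defer to the parent, and GetIdealRange returns zero radii.
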(event `self.ReceiveBeginPlay`
  (`parent.ReceiveBeginPlay`))

(event `self.ReceiveTick`
  (params (DeltaSeconds :type "Float (single-precision)"))
  (`parent.ReceiveTick` DeltaSeconds))

(event `/Game/Enemies/AI/BPI_EnemyAI.Attack`
  ;[0 0 0] Attack Damage
  (set `self.IsAttacking` true)
  (bind _asbp_aic_mud_monster_child (cast `/Game/Enemies/AI/AIControllers/BP_AIC_MudMonster_Child` (`AIBlueprintHelperLibrary.GetAIController` self)))
  (bind _attack_target (`/Game/Enemies/AI/AIControllers/BP_AIC_EnemyBasic.Attack Target` _asbp_aic_mud_monster_child)
    (:`then`
      (message `/Game/DamageSystem/BPI_Damagable.TakeDamage` _attack_target (make `/Game/DamageSystem/S_DamageInfo` 15.0 "NewEnumerator1"))
      (`KismetSystemLibrary.Delay` 0.5)
      (set `self.IsAttacking` false)
      (`self.OnAttackEnd`))
    (:`else`)))

(event `self.OnDeath`
  (`parent.OnDeath`))

(fn `GetIdealRange`
  (returns (AttackRadius :type "Float (double-precision)") (DefendRadius :type "Float (double-precision)"))
  (return 0.0 0.0))

(fn `SetMovementSpeed`
  (params (Speed :type "/Game/Enemies/AI/ENUMs/E_MovementSpeed Enum" :default "NewEnumerator0"))
  (returns (SpeedValue :type "Float (double-precision)"))
  (set `CharacterMovementComponent.MaxWalkSpeed` (select `/Game/Enemies/AI/ENUMs/E_MovementSpeed` Speed :`NewEnumerator1` 10.0 :`NewEnumerator2` 50.0 :`NewEnumerator3` 100.0 :!type "Float (single-precision)") (`self.CharacterMovement`))
  (return 0.0))

(fn `UserConstructionScript`
  (`parent.UserConstructionScript`))