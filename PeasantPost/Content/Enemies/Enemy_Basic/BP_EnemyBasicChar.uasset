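; BP_EnemyBasicChar is a sprite-based basic enemy that chases the player and deals damage on reaching them.
; ChasePlayer loops AIMoveTo into Attack, which damages the AI controller's AttackTarget.
; BPCDamageSystem backs health, healing and damage functions and a healthbar widget, while death and block events only print.
; Tick pins sprite world rotation, helpers expose speed, range, patrol and stuck state, and GetPostmanCarry is a stub returning false.
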(event `self.ReceiveBeginPlay`
  (`KismetSystemLibrary.Delay` 1.0)
  ;[0 0 0] Check if player is carrying a package - used for certain enemy atttacks.
  (`self.GetPostmanCarry`)
  ;[0 0 0] Healthbar widget creation on spawn
  (bind _returnvalue (`|CreateWidget` "/Game/DamageSystem/W_HealthbarEnemy.W_HealthbarEnemy_C" null self))
  (`WidgetComponent.SetWidget` (`self.Widget`) _returnvalue))

(event `self.ReceiveTick`
  (params (DeltaSeconds :type "Float (single-precision)"))
  ;[0 0 0] Turning sprite to camera - might be fucking up the rotation of the animation (!)
  (`|ExecutionSequence`
    (:`then_0`
      (if (`NavMovementComponent.IsMovingOnGround` (`self.CharacterMovement`))
        (set `self.IsMoving` true)
        (else
          (set `self.IsMoving` false)))
      (`SceneComponent.K2_SetWorldRotation` :`self` (`self.Sprite`)))))

(event `/Game/Enemies/AI/BPI_EnemyAI.CarryPackage`
  ;[0 0 0] Checking if player is carrying a package
  (bind _returnvalue (`GameplayStatics.GetActorOfClass` "/Game/Character/BP_Postman.BP_Postman_C"))
  (bind _iscarrying (`/Game/Character/BP_Postman.isCarrying` _returnvalue))
  (if _iscarrying
    (set `self.PostmanCarry` _iscarrying)
    (`KismetSystemLibrary.Delay` 0.5))
  (set `self.PostmanCarry` false)
  (`self.OnCarryEnd`))

(event `ChasePlayer`
  (bind (_returnvalue_x _returnvalue_y _returnvalue_z) (`KismetMathLibrary.BreakVector` (`self.GetVelocity` self)))
  (bind (_returnvalue_x_2 _returnvalue_y_2) (`KismetMathLibrary.BreakVector` (`KismetMathLibrary.Normal` (`KismetMathLibrary.MakeVector` _returnvalue_x _returnvalue_y _returnvalue_z))))
  ;[0 0 0] Chase Player
  (`|AIMoveTo` self (0.0 0.0 0.0) (`GameplayStatics.GetPlayerCharacter` 0) 25.0
    (:`OnSuccess`
      (set `self.Directionality` (`KismetMathLibrary.MakeVector2D` _returnvalue_x_2 _returnvalue_y_2))
      (`self.Attack` self)
      (`KismetSystemLibrary.Delay` 1.0)
      (`self.ChasePlayer`))))

(event `/Game/Enemies/AI/BPI_EnemyAI.Attack`
  ;[0 0 0] Attack
  (set `self.IsAttacking` true)
  (bind _asbp_aic_enemy_basic (cast `/Game/Enemies/AI/AIControllers/BP_AIC_EnemyBasic` (`AIBlueprintHelperLibrary.GetAIController` self)))
  (bind _attack_target (`/Game/Enemies/AI/AIControllers/BP_AIC_EnemyBasic.Attack Target` _asbp_aic_enemy_basic)
    (:`then`
      (message `/Game/DamageSystem/BPI_Damagable.TakeDamage` _attack_target (make `/Game/DamageSystem/S_DamageInfo` 10.0 "NewEnumerator1"))
      (`KismetSystemLibrary.Delay` 0.5)
      (set `self.IsAttacking` false)
      (`self.OnAttackEnd`))
    (:`else`)))

(event `/Game/Enemies/AI/BPI_EnemyAI.EquipWeapon`)

(event `/Game/Enemies/AI/BPI_EnemyAI.UnequipWeapon`)

(event `OnDeath_Event`
  ;[0 0 0] Damage System interface functions
  (`KismetSystemLibrary.PrintString` "BP Enemy Basic: Enemy Has Died"))

(event `Death`
  ;[0 0 0] Damage System interface functions
  (`KismetSystemLibrary.PrintString` "BP Enemy Basic: Dead"))

(event `Blocked`
  (params (CanBeParried :type Boolean))
  ;[0 0 0] Damage System interface functions
  (`KismetSystemLibrary.PrintString` "BP Enemy Basic: Blocked Attack"))

(event `Damage Response`
  (params (`Damage Response` :type "/Game/DamageSystem/E_DamageResponse Enum" :default "NewEnumerator0"))
  ;[0 0 0] Damage System interface functions
)

(fn `GetCurrentHealth`
  (returns (Health :type "Float (double-precision)"))
  (return (`/Game/DamageSystem/BPC_DamageSystem.Health` (`self.BPC_DamageSystem`))))

(fn `GetIdealRange`
  (returns (AttackRadius :type "Float (double-precision)") (DefendRadius :type "Float (double-precision)"))
  (return 20.0 200.0))

(fn `GetMaxHealth`
  (returns (GetMaxHealth :type "Float (double-precision)"))
  (return (`/Game/DamageSystem/BPC_DamageSystem.MaxHealth` (`self.BPC_DamageSystem`))))

(fn `GetPatrolRoute`
  (returns (PatrolRoute :type "/Game/Enemies/AI/BP_PatrolRoute Object Reference"))
  (return (`self.PatrolRoute`)))

(fn `GetPostmanCarry`
  (returns (PostmanCarry :type Boolean))
  (return false))

(fn `Heal`
  (params (Amount :type "Float (double-precision)"))
  (returns (NewHealth :type "Float (double-precision)"))
  (bind _newhealth (`/Game/DamageSystem/BPC_DamageSystem.Heal` (`self.BPC_DamageSystem`) Amount))
  (return _newhealth))

(fn `IsDead`
  (returns (`Is Dead` :type Boolean))
  (return (`/Game/DamageSystem/BPC_DamageSystem.IsDead` (`self.BPC_DamageSystem`))))

(fn `IsStuck`
  (returns (IsStuck :type Boolean))
  (return (and (`self.IsMoving`) (< (`KismetMathLibrary.VSize` (`self.GetVelocity`)) (`self.StuckThreshold`)))))

(fn `SetMovementSpeed`
  (params (Speed :type "/Game/Enemies/AI/ENUMs/E_MovementSpeed Enum" :default "NewEnumerator0"))
  (returns (SpeedValue :type "Float (double-precision)"))
  (bind _output_get (set `CharacterMovementComponent.MaxWalkSpeed` (select `/Game/Enemies/AI/ENUMs/E_MovementSpeed` Speed :`NewEnumerator1` 100.0 :`NewEnumerator2` 300.0 :`NewEnumerator3` 500.0 :!type "Float (single-precision)") (`self.CharacterMovement`)))
  (return _output_get))

(fn `SetVisibility`
  (params (VisibilityEnum :type "/Game/Enemies/AI/ENUMs/E_Visibility Enum" :default "NewEnumerator1"))
  (returns (VisibilityBool :type Boolean))
  (bind _output_get (set `self.IsVisible` (select `/Game/Enemies/AI/ENUMs/E_Visibility` VisibilityEnum :`NewEnumerator1` true)))
  (return _output_get))

(fn `TakeDamage`
  (params (DamageInfor :type "/Game/DamageSystem/S_DamageInfo Structure"))
  (returns (WasDamaged :type Boolean))
  (bind _wasdamaged (`/Game/DamageSystem/BPC_DamageSystem.TakeDamage` (`self.BPC_DamageSystem`) DamageInfor))
  (return _wasdamaged))

(fn `UserConstructionScript`
  (bind _bpc_damagesystem (`self.BPC_DamageSystem`))
  (set `/Game/DamageSystem/BPC_DamageSystem.MaxHealth` 100.0 _bpc_damagesystem)
  (set `/Game/DamageSystem/BPC_DamageSystem.Health` 100.0 _bpc_damagesystem)
  (add `/Game/DamageSystem/BPC_DamageSystem.OnDeath` _bpc_damagesystem (`|CreateDelegate` :!event `Death`))
  (add `/Game/DamageSystem/BPC_DamageSystem.OnBlocked` _bpc_damagesystem (`|CreateDelegate` :!event `Blocked`))
  (add `/Game/DamageSystem/BPC_DamageSystem.OnDamageResponse` _bpc_damagesystem (`|CreateDelegate` :!event `Damage Response`)))