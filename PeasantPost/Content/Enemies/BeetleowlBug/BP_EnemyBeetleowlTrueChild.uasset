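; BP_EnemyBeetleowlTrueChild is a Beetleowl bug enemy character that supplies attack, range, speed and patrol data for enemy behavior.
; Its Attack event raises an attacking flag for a brief delay, then clears it and signals attack end.
; Overridable functions return attack and defend radii and its patrol route, and map speed states to CharacterMovement max walk speed.
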(event `/Game/Enemies/AI/BPI_EnemyAI.Attack`
  (set `self.IsAttacking` true)
  (`KismetSystemLibrary.Delay` 0.5)
  (set `self.IsAttacking` false)
  (`self.OnAttackEnd`))

(fn `GetIdealRange`
  (returns (AttackRadius :type "Float (double-precision)") (DefendRadius :type "Float (double-precision)"))
  (return 25.0 125.0))

(fn `GetPatrolRoute`
  (returns (PatrolRoute :type "/Game/Enemies/AI/BP_PatrolRoute Object Reference"))
  (return (`self.PatrolRoute`)))

(fn `SetMovementSpeed`
  (params (Speed :type "/Game/Enemies/AI/ENUMs/E_MovementSpeed Enum" :default "NewEnumerator0"))
  (returns (SpeedValue :type "Float (double-precision)"))
  (bind _output_get (set `CharacterMovementComponent.MaxWalkSpeed` (select `/Game/Enemies/AI/ENUMs/E_MovementSpeed` Speed :`NewEnumerator1` 100.0 :`NewEnumerator2` 300.0 :`NewEnumerator3` 500.0 :!type "Float (single-precision)") (`self.CharacterMovement`)))
  (return _output_get))

(fn `UserConstructionScript`
  (`parent.UserConstructionScript`))