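; Basic enemy character that chases the first player and flags an attack on reaching them.
; A looping AI MoveTo stores normalized XY velocity as Directionality on success, sets IsAttacking, then clears it after a delay and chases again.
; A failed move has no retry.
; An IsStuck speed check is defined but uncalled, the IsMoving velocity logic appears unwired, and the sprite-facing attempt is marked broken.
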(event `self.ReceiveBeginPlay`
  (`self.ChasePlayer`)
  ;[0 0 0] Trying to turn sprite to camera (not working)
  (`SceneComponent.K2_SetWorldRotation` (`self.Sprite`) (struct) false false))

(event `ChasePlayer`
  (bind (_returnvalue_x _returnvalue_y _returnvalue_z) (`KismetMathLibrary.BreakVector` (`self.GetVelocity` self)))
  (bind (_returnvalue_x_2 _returnvalue_y_2) (`KismetMathLibrary.BreakVector` (`KismetMathLibrary.Normal` (`KismetMathLibrary.MakeVector` _returnvalue_x _returnvalue_y _returnvalue_z))))
  ;[0 0 0] Chase Player
  (`|AIMoveTo` self (0.0 0.0 0.0) (`GameplayStatics.GetPlayerCharacter` 0) 25.0
    (:`OnSuccess`
      (set `self.Directionality` (`KismetMathLibrary.MakeVector2D` _returnvalue_x_2 _returnvalue_y_2))
      (`self.Attack` self)
      (`KismetSystemLibrary.Delay` 1.0)
      (set `self.IsAttacking` false)
      (`self.ChasePlayer`))))

(event `Attack`
  (set `self.IsAttacking` true))

(fn `IsStuck`
  (returns (IsStuck :type Boolean))
  (return (and (`self.IsMoving`) (< (`KismetMathLibrary.VSize` (`self.GetVelocity`)) (`self.StuckThreshold`)))))

(fn `UserConstructionScript`)