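; Basic enemy character with a sprite that chases the first player's character through AI movement.
; BeginPlay starts the chase and zeroes the sprite's world rotation; ChasePlayer reissues AIMoveTo on a repeating delay, storing normalized velocity XY as Directionality each pass.
; Move success or failure sets IsMoving, which IsStuck combines with a low-speed threshold to detect a stuck enemy, though this Blueprint never calls that check.
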(event `self.ReceiveBeginPlay`
  (`self.ChasePlayer`)
  (`SceneComponent.K2_SetWorldRotation` :`self` (`self.Sprite`)))

(event `ChasePlayer`
  (bind (_returnvalue_x _returnvalue_y _returnvalue_z) (`KismetMathLibrary.BreakVector` (`self.GetVelocity` self)))
  (bind (_returnvalue_x_2 _returnvalue_y_2) (`KismetMathLibrary.BreakVector` (`KismetMathLibrary.Normal` (`KismetMathLibrary.MakeVector` _returnvalue_x _returnvalue_y _returnvalue_z))))
  ;[0 0 0] Chase Player
  (`|AIMoveTo` self (0.0 0.0 0.0) (`GameplayStatics.GetPlayerCharacter` 0)
    (:`then`
      (set `self.Directionality` (`KismetMathLibrary.MakeVector2D` _returnvalue_x_2 _returnvalue_y_2))
      (`KismetSystemLibrary.Delay` 2.0)
      (`self.ChasePlayer`))
    (:`OnSuccess`
      (set `self.IsMoving` true))
    (:`OnFail`
      (set `self.IsMoving` false))))

(fn `IsStuck`
  (returns (IsStuck :type Boolean))
  (return (and (`self.IsMoving`) (< (`KismetMathLibrary.VSize` (`self.GetVelocity`)) (`self.StuckThreshold`)))))

(fn `UserConstructionScript`)