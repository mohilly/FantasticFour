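; AI controller for basic and ranged enemies that runs the pawn's behaviour tree and drives its blackboard combat state.
; On possess it sets Passive; attack and defend radii come from the pawn's ideal-range message.
; Perception updates attack the player on sight, or any damage-sensed actor when Passive or Investigating.
; The sight handler switches on a literal Passive, ignoring the current state it reads.
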(event `self.ReceivePossess`
  (params (PossessedPawn :type "Pawn Object Reference"))
  (bind _asbp_enemy_basic_char (cast `/Game/Enemies/Enemy_Basic/BP_EnemyBasicChar` PossessedPawn)
    (:`then`
      (bind _behaviourtree (`/Game/Enemies/Enemy_Basic/BP_EnemyBasicChar.BehaviourTree` _asbp_enemy_basic_char)
        (:`then`
          (`self.RunBehaviorTree` _behaviourtree)
          (`self.SetStateAsPassive` :!label _label)
          (bind (_attackradius _defendradius) (message `/Game/Enemies/AI/BPI_EnemyAI.GetIdealRange` PossessedPawn))
          (`BlackboardComponent.SetValueAsFloat` (`self.Blackboard`) (`self.Attack Radius Key Name`) _attackradius)
          (`BlackboardComponent.SetValueAsFloat` (`self.Blackboard`) (`self.Defend Radius Key Name`) _defendradius))
        (:`else`
          (`KismetSystemLibrary.PrintString` "No valid behaviour treee in enemy actor"))))
    (:`CastFailed`
      (bind _asbp_enemy_ranged (cast `/Game/Enemies/Enemy_Ranged/BP_EnemyRanged` PossessedPawn))
      (bind _behaviourtree_2 (`/Game/Enemies/Enemy_Basic/BP_EnemyBasicChar.BehaviourTree` _asbp_enemy_ranged)
        (:`then`
          (`self.RunBehaviorTree` _behaviourtree_2)
          (goto _label))
        (:`else`)))))

(event `self.AIPerception.OnPerceptionUpdated`
  (params (UpdatedActors :type "Array of Actor Object Reference (by ref)"))
  (for _array_element UpdatedActors
    (`|ExecutionSequence`
      (:`then_0`
        ;[0 0 0] Reaction on Sight
        (bind _sensed (`self.CanSenseActor` _array_element "NewEnumerator1"))
        (if _sensed
          (`self.HandleSensedSight` _array_element)))
      (:`then_1`
        ;[0 0 0] Reaction on Damage
        (bind _sensed_2 (`self.CanSenseActor` _array_element "NewEnumerator2"))
        (if _sensed_2
          (`self.HandleSensedDamage` _array_element))))))

(fn `CanSenseActor`
  (params (Actor :type "Actor Object Reference") (Sense :type "/Game/Enemies/AI/ENUMs/E_AISense Enum" :default "NewEnumerator0"))
  (returns (Sensed :type Boolean) (Stimulus :type "AIStimulus Structure"))
  (bind _info (`AIPerceptionComponent.GetActorsPerception` (`self.AIPerception`) Actor))
  (for _array_element (`.LastSensedStimuli` (break `ActorPerceptionBlueprintInfo` _info))
    (bind _returnvalue (`AIPerceptionSystem.GetSenseClassForStimulus` _array_element))
    (if (== _returnvalue (select `/Game/Enemies/AI/ENUMs/E_AISense` Sense :`NewEnumerator1` "/Script/AIModule.AISense_Sight" :`NewEnumerator2` "/Script/AIModule.AISense_Damage" :!type "Object Class Reference"))
      (return (`.bSuccessfullySensed` (break `AIStimulus` _array_element)) _array_element))))

(fn `GetCurrentState`
  (returns (State :type "/Game/Enemies/AI/ENUMs/E_EnemyStates Enum"))
  (return (cast `/Game/Enemies/AI/ENUMs/E_EnemyStates` (`BlackboardComponent.GetValueAsEnum` (`self.Blackboard`) (`self.Enemy States Key Name`)))))

(fn `HandleSensedDamage`
  (params (Actor :type "Actor Object Reference"))
  (bind _state (`self.GetCurrentState`))
  (switch `/Game/Enemies/AI/ENUMs/E_EnemyStates` _state
    (:`NewEnumerator0`
      _)
    (:`NewEnumerator3`
      _))
  (`self.SetStateAsAttacking` Actor))

(fn `HandleSensedSight`
  (params (Actor :type "Actor Object Reference"))
  (`self.GetCurrentState`)
  (switch `/Game/Enemies/AI/ENUMs/E_EnemyStates` "NewEnumerator0"
    (:`NewEnumerator0`
      _)
    (:`NewEnumerator3`
      _))
  (if (== Actor (`GameplayStatics.GetPlayerCharacter` 0))
    (`self.SetStateAsAttacking` Actor)))

(fn `SetStateAsAttacking`
  (params (AttackTarget :type "Actor Object Reference"))
  (`BlackboardComponent.SetValueAsObject` (`self.Blackboard`) (`self.Attack Target Key Name`) AttackTarget)
  (`BlackboardComponent.SetValueAsEnum` (`self.Blackboard`) (`self.Enemy States Key Name`) (enumliteral `/Game/Enemies/AI/ENUMs/E_EnemyStates` "NewEnumerator1"))
  (set `self.Attack Target` AttackTarget))

(fn `SetStateAsPassive`
  (`BlackboardComponent.SetValueAsEnum` (`self.Blackboard`) (`self.Enemy States Key Name`) (enumliteral `/Game/Enemies/AI/ENUMs/E_EnemyStates` "NewEnumerator0")))

(fn `UserConstructionScript`)