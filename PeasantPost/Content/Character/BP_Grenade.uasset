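; BP_Grenade is a grenade projectile that flies to a target point and explodes.
; Tick moves it toward VectorTo with constant-speed interpolation from a slightly raised position, triggering BlowUp on arrival.
; Sphere overlaps also detonate it once the OverlapTimer arming countdown expires.
; Detonation enables the hidden Explosion's query collision, swaps visibility with the render component, then uses DoOnce to play a sound and destroy the actor after a delay.
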(event `self.ReceiveBeginPlay`
  (`PrimitiveComponent.SetCollisionEnabled` (`self.Explosion`) "NoCollision"))

(event `self.ReceiveTick`
  (params (DeltaSeconds :type "Float (single-precision)"))
  (`self.K2_SetActorLocation` (`KismetMathLibrary.VInterpTo_Constant` (+ (`self.K2_GetActorLocation`) (0.0 0.0 5.0)) (`self.vectorTo`) DeltaSeconds (`self.speed`)))
  (set `self.overlapTimer` (- (`self.overlapTimer`) DeltaSeconds))
  (if (== (`self.vectorTo`) (`self.K2_GetActorLocation`) :`ErrorTolerance` 0.5)
    (`self.Blow Up`)))

(event `Blow Up`
  (`PrimitiveComponent.SetCollisionEnabled` (`self.Explosion`) "QueryOnly" :!label _label)
  (`SceneComponent.SetHiddenInGame` (`self.Explosion`) false false)
  (`SceneComponent.SetHiddenInGame` (`self.RenderComponent`) true false)
  (`/Engine/EditorBlueprintResources/StandardMacros.DoOnce` false
    (:`Completed`
      (`FMODBlueprintStatics.PlayEventAtLocation` "/Game/FMOD/Events/SFX/SFX_EXPLOSION.SFX_EXPLOSION" (`SceneComponent.K2_GetComponentToWorld` (`self.Explosion`)))
      (`KismetSystemLibrary.Delay` (`self.explosionLength`))
      (`self.K2_DestroyActor`))))

(event `self.CollisionSphere.OnComponentBeginOverlap`
  (params (OverlappedComponent :type "PrimitiveComponent Object Reference") (OtherActor :type "Actor Object Reference") (OtherComp :type "PrimitiveComponent Object Reference") (OtherBodyIndex :type Integer) (bFromSweep :type Boolean) (SweepResult :type "HitResult Structure (by ref)"))
  (if (<= (`self.overlapTimer`) 0.0)
    (goto _label)))

(fn `UserConstructionScript`)