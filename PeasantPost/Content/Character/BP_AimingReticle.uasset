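; A possessable aiming reticle that the player steers around its parent character while the view target stays on that character.
; Move input adjusts a range-limited X/Y offset, which Tick adds to the parent's location, also setting the parent's left/right Directionality from reticle position and OnReturn.
; The action input briefly reveals a sphere, gated by a cooldown.
; Pressing P clears OnReturn, repossesses the parent and destroys the reticle.
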(event `self.ReceiveBeginPlay`
  (bind _asplayer_controller (cast `PlayerController` (`self.GetController`)))
  (`EnhancedInputSubsystemInterface.AddMappingContext` (pcsubsystem `EnhancedInputLocalPlayerSubsystem` _asplayer_controller) "/Game/Character/Input/IMC_TopDown.IMC_TopDown" 0 (struct)))

(event `EnhancedInput|/Game/Character/Input/IA_Move`
  (params (ActionValue :type "Vector2D Structure") (ElapsedSeconds :type "Float (double-precision)") (TriggeredSeconds :type "Float (double-precision)") (InputAction :type "InputAction Object Reference" :default "/Game/Character/Input/IA_Move.IA_Move"))
  (bind _roffsetmax (`self.rOffsetMax`))
  (bind _roffsetmax_2 (`self.rOffsetMax`))
  (bind _returnvalue (+ (`self.rOffsetY`) (* (`self.rOffsetIncrement`) (* ActionValue_Y -1.0))))
  (bind _returnvalue_2 (+ (`self.rOffsetX`) (* (`self.rOffsetIncrement`) ActionValue_X)))
  (:`Triggered`
    (if (`KismetMathLibrary.InRange_FloatFloat` _returnvalue_2 (* -1.0 _roffsetmax_2) _roffsetmax_2)
      (set `self.rOffsetX` _returnvalue_2))
    (if (`KismetMathLibrary.InRange_FloatFloat` _returnvalue (* -1.0 _roffsetmax) _roffsetmax)
      (set `self.rOffsetY` _returnvalue))))

(event `Key|P`
  (params (Key :type "Key Structure"))
  (bind _playerparent (`self.playerParent`))
  (:`Pressed`
    (set `/Game/Character/BP_Postman.onReturn` false _playerparent)
    (`Controller.Possess` (`self.GetController`) _playerparent)
    (`self.K2_DestroyActor`)))

(event `self.ReceiveTick`
  (params (DeltaSeconds :type "Float (single-precision)"))
  (bind _returnvalue_x (`KismetMathLibrary.BreakVector` (`self.K2_GetActorLocation`)))
  (bind (_returnvalue_x_2 _returnvalue_y _returnvalue_z) (`KismetMathLibrary.BreakVector` (`self.K2_GetActorLocation`)))
  (bind _playerparent (`self.playerParent`))
  (bind _playerparent_2 (`self.playerParent`))
  (bind (_returnvalue_x_3 _returnvalue_y_2) (`KismetMathLibrary.BreakVector` (`self.K2_GetActorLocation` _playerparent_2)))
  (bind _returnvalue_x_4 (`KismetMathLibrary.BreakVector` (`self.K2_GetActorLocation` _playerparent)))
  ;[0.037 0.037 0.037] set camera to player character
  (`PlayerController.SetViewTargetWithBlend` (`GameplayStatics.GetPlayerController` 0) _playerparent_2 0.0 "VTBlend_Linear" 0.0 false)
  (`self.K2_SetActorLocation` (`KismetMathLibrary.MakeVector` (+ _returnvalue_x_3 (`self.rOffsetX`)) (+ _returnvalue_y_2 (`self.rOffsetY`)) _returnvalue_z))
  (if (and (> _returnvalue_x _returnvalue_x_4) (`/Game/Character/BP_Postman.onReturn` _playerparent))
    (set `/Game/Character/BP_Postman.Directionality` (1.0 0.0) _playerparent)
    (else
      (set `/Game/Character/BP_Postman.Directionality` (-1.0 0.0) _playerparent))))

(event `EnhancedInput|/Game/Character/Input/IA_Action`
  (params (ActionValue :type Boolean) (ElapsedSeconds :type "Float (double-precision)") (TriggeredSeconds :type "Float (double-precision)") (InputAction :type "InputAction Object Reference" :default "/Game/Character/Input/IA_Action.IA_Action"))
  (bind _sphere (`self.Sphere`))
  (:`Started`
    (if (`self.canFire`)
      (`SceneComponent.SetHiddenInGame` _sphere false false)
      (set `self.canFire` false)
      (`KismetSystemLibrary.Delay` 0.5)
      (`SceneComponent.SetHiddenInGame` _sphere true false)
      (set `self.canFire` true))))

(fn `UserConstructionScript`)