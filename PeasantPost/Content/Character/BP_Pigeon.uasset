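; Companion pigeon that follows the postman player, or circles the cart when its OnWagon flag is set.
; Tick interpolates it toward a point near the player until it perches, or around an angle-stepped orbit sized by its sphere radius.
; An attack halts movement for a frame-counted timer, showing the hitbox and only printing overlapping enemies.
; Afterwards its interp speed drops and ramps back up, so it catches up gradually.
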(event `self.ReceiveTick`
  (params (DeltaSeconds :type "Float (single-precision)"))
  (if (`self.isAttacking`)
    (`self.Pigeon Attack`)
    (else
      (if (`self.isPostAttack`)
        (`self.Pigeon Attack Rcovery`))
      (if (not (`self.onWagon`))
        (bind _returnvalue (`self.Check If On Player`))
        (bind _output_get (set `self.onPostman` _returnvalue))
        (if _output_get
          (set `self.interpSpeed` (`self.interpSpeedTrue`))
          (set `self.isPostAttack` false)
          (else
            (bind _returnvalue_2 (`self.Move to Player Location` DeltaSeconds))
            (`self.K2_SetActorLocation` _returnvalue_2)))
        (else
          (`self.Increment Angle`)
          (bind _returnvalue_3 (`GameplayStatics.GetActorOfClass` "/Game/Mia/BP_CartMovement.BP_CartMovement_C"))
          (bind _newvector (`self.Movement on Radius` _returnvalue_3 DeltaSeconds))
          (`self.K2_SetActorLocation` _newvector)))
      ;[1 1 1] For Testing
      (`SceneComponent.SetHiddenInGame` (`self.Hitbox`) true false))))

(event `self.ReceiveBeginPlay`
  (set `self.interpSpeed` (`self.interpSpeedTrue`))
  (set `self.attackTimer` (`self.attackTimerTrue`))
  (bind _asbp_postman (cast `/Game/Character/BP_Postman` (`GameplayStatics.GetPlayerCharacter` 0)))
  (set `self.varPostman` _asbp_postman))

(fn `Check If On Player`
  (returns (ReturnValue :type Boolean))
  (bind (_returnvalue_x _returnvalue_y _returnvalue_z) (`KismetMathLibrary.BreakVector` (`self.K2_GetActorLocation` (`self.varPostman`))))
  (bind (_returnvalue_x_2 _returnvalue_y_2 _returnvalue_z_2) (`KismetMathLibrary.BreakVector` (- (`self.K2_GetActorLocation`) (2.0 2.0 30.0))))
  (return (and (`KismetMathLibrary.InRange_FloatFloat` _returnvalue_x_2 (- _returnvalue_x 0.2) (+ _returnvalue_x 0.2)) (`KismetMathLibrary.InRange_FloatFloat` _returnvalue_y_2 (- _returnvalue_y 0.2) (+ _returnvalue_y 0.2)) (`KismetMathLibrary.InRange_FloatFloat` _returnvalue_z_2 (- _returnvalue_z 0.2) (+ _returnvalue_z 0.2)))))

(fn `Hitcheck`
  (for _array_element (`PrimitiveComponent.GetOverlappingActors` (`self.Hitbox`) "/Game/Enemies/Enemy_Basic/BP_EnemyBasicChar.BP_EnemyBasicChar_C")
    (`KismetSystemLibrary.PrintString` (`KismetSystemLibrary.GetPathName` _array_element))))

(fn `Increment Angle`
  (set `self.patrolAngle` (+ (`self.patrolAngle`) 1))
  (if (> (`self.patrolAngle`) 359)
    (set `self.patrolAngle` 0.0)))

(fn `Move to Player Location`
  (params (DeltaTime :type "Float (single-precision)"))
  (returns (ReturnValue :type "Vector Structure"))
  (bind _returnvalue (`GameplayStatics.GetPlayerPawn` 0))
  (bind (_returnvalue_x _returnvalue_y _returnvalue_z) (`KismetMathLibrary.BreakVector` (`self.GetActorForwardVector` _returnvalue)))
  (return (`KismetMathLibrary.VInterpTo` (`self.K2_GetActorLocation`) (+ (`self.K2_GetActorLocation` _returnvalue) (* (`KismetMathLibrary.MakeVector` _returnvalue_x (+ _returnvalue_y 1.0) (- _returnvalue_z -15.0)) 2)) DeltaTime (`self.interpSpeed`))))

(fn `Movement on Radius`
  (params (`Cart Plane` :type "/Game/Mia/BP_CartMovement Object Reference") (DeltaTime :type "Float (double-precision)"))
  (returns (NewVector :type "Vector Structure"))
  (bind (_returnvalue_x _returnvalue_y _returnvalue_z) (`KismetMathLibrary.BreakVector` (`self.GetActorForwardVector` `Cart Plane`)))
  (bind _patrolangle (`self.patrolAngle`))
  (bind _returnvalue (`SphereComponent.GetScaledSphereRadius` (`self.Sphere`)))
  (return (`KismetMathLibrary.VInterpTo` (`self.K2_GetActorLocation`) (+ (`SceneComponent.K2_GetComponentLocation` (`/Game/Mia/BP_CartMovement.Plane ` `Cart Plane`)) (`KismetMathLibrary.MakeVector` (+ _returnvalue_x (* (`KismetMathLibrary.DegCos` _patrolangle) _returnvalue)) (+ (* _returnvalue (`KismetMathLibrary.DegSin` _patrolangle)) _returnvalue_y) (+ _returnvalue_z 100.0))) DeltaTime (`self.interpSpeed`))))

(fn `Pigeon Attack`
  ;[0 0 0] Actual Attack
  (`self.Hitcheck`)
  ;[1 1 1] For Testing
  (`SceneComponent.SetHiddenInGame` (`self.Hitbox`) false false)
  (set `self.attackTimer` (- (`self.attackTimer`) 1))
  (if (<= (`self.attackTimer`) 0)
    (set `self.isAttacking` false)
    (set `self.isPostAttack` true)
    (set `self.interpSpeed` (`self.interpSpeedPostAttack`))
    (set `self.attackTimer` (`self.attackTimerTrue`))))

(fn `Pigeon Attack Rcovery`
  ;[0 0 0] After attack, pigeon slowly catches back up to the player
  (if (< (`self.interpSpeed`) (`self.interpSpeedTrue`))
    (set `self.interpSpeed` (+ (`self.interpSpeed`) (`self.interpSpeedPostAttackIncrement`)))))

(fn `UserConstructionScript`)