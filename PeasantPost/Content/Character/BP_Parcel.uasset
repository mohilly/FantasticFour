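; Parcel actor that the postman carries and drops off, either at a delivery zone or on the wagon.
; While carried, Tick interpolates it to a point in front of the player using the postman's directionality; otherwise it runs Placed every frame.
; Placed triggers the cart's alert mode once for the main parcel on the wagon, or completes a delivery and destroys both zone and parcel.
; Health and damage functions are empty stubs.
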(event `self.ReceiveTick`
  (params (DeltaSeconds :type "Float (single-precision)"))
  (bind _returnvalue (`GameplayStatics.GetPlayerPawn` 0))
  (bind (_returnvalue_x _returnvalue_y _returnvalue_z) (`KismetMathLibrary.BreakVector` (`self.GetActorForwardVector` _returnvalue)))
  ;[0 0 0] Changing Parcel Position if being carried
  (if (`self.isCarried`)
    (bind _asbp_postman (cast `/Game/Character/BP_Postman` _returnvalue))
    (bind _directionality_x (`KismetMathLibrary.BreakVector2D` (`/Game/Character/BP_Postman.Directionality` _asbp_postman)))
    (`self.K2_SetActorLocation` (`KismetMathLibrary.VInterpTo` (`self.K2_GetActorLocation`) (+ (`self.K2_GetActorLocation` _returnvalue) (* (`KismetMathLibrary.MakeVector` (* _returnvalue_x _directionality_x) (- _returnvalue_y 1.0) _returnvalue_z) 30)) DeltaSeconds 120.0))
    (else
      (`self.Placed`))))

(event `self.ReceiveActorBeginOverlap`
  (params (OtherActor :type "Actor Object Reference"))
  (set `self.isOverlapping` true))

(event `self.ReceiveActorEndOverlap`
  (params (OtherActor :type "Actor Object Reference"))
  (set `self.isOverlapping` false))

(event `self.ReceiveBeginPlay`)

(event `Placed`
  (bind _overlappingactors (`self.GetOverlappingActors` "/Game/Mia/BP_Delivery.BP_Delivery_C"))
  ;[0 0 0] Checking if the main parcel is put on the wagon
  (if (and (`self.onWagon`) (`self.isMainParcel`))
    ;[0 0 0] Change the Cart Movement
    (`/Engine/EditorBlueprintResources/StandardMacros.DoOnce` false
      (:`Completed`
        (bind _asbp_cart_movement (cast `/Game/Mia/BP_CartMovement` (`|GetArrayItem` (`self.GetOverlappingActors` "/Game/Mia/BP_CartMovement.BP_CartMovement_C"))))
        (`/Game/Mia/BP_CartMovement.Activate Alert Mode` _asbp_cart_movement)))
    (else
      ;[0 0 0] Checking if the normal Parcel is placed in the zone
      (if (and (> (`KismetArrayLibrary.Array_Length` _overlappingactors) 0) (`self.inTheZone`))
        (`self.K2_DestroyActor` (`|GetArrayItem` _overlappingactors))
        (bind _asbp_postman (cast `/Game/Character/BP_Postman` (`GameplayStatics.GetPlayerCharacter` 0)))
        (`/Game/Character/BP_Postman.delivery` _asbp_postman)
        (`FMODBlueprintStatics.PlayEvent2D` "/Game/FMOD/Events/SFX/SFX_DELIVERY.SFX_DELIVERY")
        (`self.K2_DestroyActor`)))))

(fn `GetCurrentHealth`
  (returns (Health :type "Float (double-precision)"))
  (return 0.0))

(fn `GetMaxHealth`
  (returns (GetMaxHealth :type "Float (double-precision)"))
  (return 0.0))

(fn `Heal`
  (params (Amount :type "Float (double-precision)"))
  (returns (NewHealth :type "Float (double-precision)"))
  (return 0.0))

(fn `IsDead`
  (returns (`Is Dead` :type Boolean))
  (return false))

(fn `TakeDamage`
  (params (DamageInfor :type "/Game/DamageSystem/S_DamageInfo Structure"))
  (returns (WasDamaged :type Boolean))
  (return false))

(fn `UserConstructionScript`)